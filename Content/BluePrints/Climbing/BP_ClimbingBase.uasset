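; BP_ClimbingBase is a base Blueprint for climbable objects that tells players when they can climb.
; Entering or leaving CollisionBox toggles CanClimb on the player, passing itself as the climbing object on entry.
; UpperCollisionBox blocks climbing up while the player overlaps it and restores it on exit.
; Overlaps run only with authority, filter on the Player tag, and reach players through message calls via GetPlayerRefMessage.
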(event OnComponentBeginOverlap(CollisionBox)
  (params (OverlappedComponent :type Primitive%20Component%20Object%20Reference) (OtherActor :type Actor%20Object%20Reference) (OtherComp :type Primitive%20Component%20Object%20Reference) (OtherBodyIndex :type Integer) (bFromSweep :type Boolean) (SweepResult :type Hit%20Result%20Structure%20%28by%20ref%29))
  (Networking|SwitchHasAuthority
    (:Authority
      (if (Actor|ActorHasTag OtherActor "Player")
        (bind _player (Class|INTPlayerBase|GetPlayerRef(Message) OtherActor))
        (Default|CanClimb _player true self)))))

(event OnComponentEndOverlap(CollisionBox)
  (params (OverlappedComponent :type Primitive%20Component%20Object%20Reference) (OtherActor :type Actor%20Object%20Reference) (OtherComp :type Primitive%20Component%20Object%20Reference) (OtherBodyIndex :type Integer))
  (Networking|SwitchHasAuthority
    (:Authority
      (if (Actor|ActorHasTag OtherActor "Player")
        (bind _player (Class|INTPlayerBase|GetPlayerRef(Message) OtherActor))
        (Default|CanClimb _player false)))))

(event OnComponentBeginOverlap(UpperCollisionBox)
  (params (OverlappedComponent :type Primitive%20Component%20Object%20Reference) (OtherActor :type Actor%20Object%20Reference) (OtherComp :type Primitive%20Component%20Object%20Reference) (OtherBodyIndex :type Integer) (bFromSweep :type Boolean) (SweepResult :type Hit%20Result%20Structure%20%28by%20ref%29))
  (Networking|SwitchHasAuthority
    (:Authority
      (if (Actor|ActorHasTag OtherActor "Player")
        (bind _player (Class|INTPlayerBase|GetPlayerRef(Message) OtherActor))
        (Class|INTPlayerBase|SetCanClimbUp(Message) _player false)))))

(event OnComponentEndOverlap(UpperCollisionBox)
  (params (OverlappedComponent :type Primitive%20Component%20Object%20Reference) (OtherActor :type Actor%20Object%20Reference) (OtherComp :type Primitive%20Component%20Object%20Reference) (OtherBodyIndex :type Integer))
  (Networking|SwitchHasAuthority
    (:Authority
      (if (Actor|ActorHasTag OtherActor "Player")
        (bind _player (Class|INTPlayerBase|GetPlayerRef(Message) OtherActor))
        (Class|INTPlayerBase|SetCanClimbUp(Message) _player true)))))

(fn ConstructionScript)