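; Base 2D flipbook enemy for a networked game, with health, damage and animations held in an EnemyInfo struct.
; Server events set MovementState, whose RepNotify swaps the Idle, Move, Hit or Death flipbook.
; Taking damage lowers health, plays the hit reaction, stops AI logic, then starts a looping AIMoveTo chase of the instigator.
; Player overlap on the authority runs a repeating timer that damages overlapping players not in GodMode.
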(event OnComponentBeginOverlap(Collision)
  (params (OverlappedComponent :type Primitive%20Component%20Object%20Reference) (OtherActor :type Actor%20Object%20Reference) (OtherComp :type Primitive%20Component%20Object%20Reference) (OtherBodyIndex :type Integer) (bFromSweep :type Boolean) (SweepResult :type Hit%20Result%20Structure%20%28by%20ref%29))
  (Networking|SwitchHasAuthority
    (:Authority
      (if (Actor|ActorHasTag OtherActor "Player")
        (CallFunction|StartApplyDamage true)))))

(event OnComponentEndOverlap(Collision)
  (params (OverlappedComponent :type Primitive%20Component%20Object%20Reference) (OtherActor :type Actor%20Object%20Reference) (OtherComp :type Primitive%20Component%20Object%20Reference) (OtherBodyIndex :type Integer))
  (Networking|SwitchHasAuthority
    (:Authority
      (if (Actor|ActorHasTag OtherActor "Player")
        (CallFunction|StartApplyDamage false)))))

(event Custom|SRV_SetMovementState
  (params (MovementState :type E_MovementState%20Enum :default "NewEnumerator0"))
  (Variables|Default|SetMovementState MovementState))

(event Custom|SRV_StartApplyDamage
  (params (bApplyDamage :type Boolean))
  (if bApplyDamage
    (bind _returnvalue (Utilities|Time|SetTimerbyEvent (delegate Custom|ApplyDamage) 0.1 true))
    (Variables|Default|SetApplyDamageHandle _returnvalue)
    (else
      (Utilities|Time|ClearandInvalidateTimerbyHandle (Variables|Default|GetApplyDamageHandle)))))

(event Custom|ApplyDamage
  (for _array_element (Collision|GetOverlappingActors "/Game/BluePrints/Player/BP_PlayerBase.BP_PlayerBase_C" :!class /Script/Engine.Actor)
    (bind _player (Class|INTPlayerBase|GetPlayerRef(Message) _array_element))
    (if (not (Variables|/Game/BluePrints/Player/BP_PlayerBase.BP_PlayerBase_C|GetbGodMode _player))
      (Game|Damage|ApplyDamage _player (.Damage (Utilities|Struct|BreakST_EnemyInfo (Variables|Default|GetEnemyInfo))) (Pawn|GetController) 0))))

(event EventSetMovementState
  (params (MovementStates :type E_MovementState%20Enum :default "NewEnumerator0"))
  (CallFunction|SRVSetMovementState MovementStates))

(event Game|Damage|EventAnyDamage
  (params (Damage :type Float%20%28single-precision%29) (DamageType :type Damage%20Type%20Object%20Reference) (InstigatedBy :type Controller%20Object%20Reference) (DamageCauser :type Actor%20Object%20Reference))
  (bind _returnvalue (Transformation|GetActorLocation))
  (bind (_x _y _z) (Math|Vector|BreakVector _returnvalue))
  (Variables|Default|SetPlayerController InstigatedBy)
  (CallFunction|SetMovementState "NewEnumerator6")
  (Pawn|Components|CharacterMovement|SetMovementMode (Variables|Character|GetCharacterMovement) "MOVE_None" 0)
  (bind _structout (Utilities|Struct|SetmembersinST_EnemyInfo (Variables|Default|GetEnemyInfo) (Math|Float|Clamp(Float) (- (.Health (Utilities|Struct|BreakST_EnemyInfo (Variables|Default|GetEnemyInfo))) Damage) 0.0 (.Health (Utilities|Struct|BreakST_EnemyInfo (Variables|Default|GetEnemyInfo))))))
  (Variables|Default|SetEnemyInfo _structout)
  (Utilities|FlowControl|Delay (Class|PaperFlipbookComponent|GetFlipbookLength (Variables|Default|GetSprite)))
  (Components|Movement|StopMovementImmediately (Variables|Character|GetCharacterMovement))
  (bind _aicontroller (Class|INTAIController|GetAIControllerRef(Message) (Pawn|GetController)))
  (AI|Logic|StopLogic (Variables|/Script/AIModule.AIController|GetBrainComponent _aicontroller) "Hit")
  (Pawn|Components|CharacterMovement|SetMovementMode (Variables|Character|GetCharacterMovement) "MOVE_Walking" 0)
  (CallFunction|SetMovementState "NewEnumerator1")
  (AI|AIMoveTo self (Transformation|GetActorLocation (Pawn|GetControlledPawn (Variables|Default|GetPlayerController))) (Pawn|GetControlledPawn (Variables|Default|GetPlayerController)) 2.0 false :!label _label
    (:then
      (AI|AIMoveTo (AI|GetAIController self) (Math|Vector|MakeVector (+ _x (Math|Float|SelectFloat -125.0 125.0 (< (.X (Math|Vector|BreakVector (Transformation|GetActorLocation (Pawn|GetControlledPawn (Variables|Default|GetPlayerController))))) _x))) _y _z) 0 -1.0 "Default" "Default" true true
        (:OnMoveFinished
          (goto _label))))))

(event EventStartApplyDamage
  (params (bApplyDamage :type Boolean))
  (CallFunction|SRVStartApplyDamage bApplyDamage))

(fn ConstructionScript
  (|CallParentFunction))

(fn OnRepBIsMoving
  (bind _sprite (Variables|Default|GetSprite))
  (bind _enemyinfo (Variables|Default|GetEnemyInfo))
  (bind (_name _health _damage _idleanim _moveanim) (Utilities|Struct|BreakST_EnemyInfo _enemyinfo))
  (if (not (Variables|Default|GetbIsMoving))
    (Sprite|SetFlipbook _sprite _idleanim)
    (else
      (Sprite|SetFlipbook _sprite _moveanim))))

(fn OnRepMovementState
  (bind _enemyinfo (Variables|Default|GetEnemyInfo))
  (bind (_name _damage _idleanim _moveanim _hitanim _deathanim) (Utilities|Struct|BreakST_EnemyInfo _enemyinfo))
  (switch Utilities|FlowControl|Switch|SwitchonE_MovementState (Variables|Default|GetMovementState)
    (:NewEnumerator0
      (Sprite|SetFlipbook (Variables|Default|GetSprite) _idleanim))
    (:NewEnumerator1
      (Sprite|SetFlipbook (Variables|Default|GetSprite) _moveanim))
    (:NewEnumerator6
      (Sprite|SetFlipbook (Variables|Default|GetSprite) _hitanim))
    (:NewEnumerator7
      (Sprite|SetFlipbook (Variables|Default|GetSprite) _deathanim))))

(fn GetEnemyRef
  (return self))